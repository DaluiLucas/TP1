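; BP8TESTConstr is a test actor that draws a diagonal row of debug line traces sized by its Box component.
; The construction script sets a fixed cubic extent on the Box.
; On BeginPlay a loop steps TempX and TempY by DistTrace until both exceed the extent, tracing vertically on Visibility with persistent drawing.
; Trace points ignore the actor's location, and the hit results go unused.
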(event `self.ReceiveBeginPlay`
  (bind _tempx (`self.TempX`))
  (bind _tempy (`self.TempY`))
  (bind _disttrace (`self.DistTrace`))
  (while (`KismetMathLibrary.BooleanNAND` (> _tempx (.x (`BoxComponent.GetScaledBoxExtent` (`self.Box`)))) (> _tempy (.y (`BoxComponent.GetScaledBoxExtent` (`self.Box`)))))
    (`KismetSystemLibrary.LineTraceSingle` :`Start` (`KismetMathLibrary.MakeVector` _tempx _tempy (.z (`BoxComponent.GetScaledBoxExtent` (`self.Box`)))) :`End` (`KismetMathLibrary.MakeVector` _tempx _tempy -5.0) :`TraceChannel` "TraceTypeQuery1" :`DrawDebugType` "Persistent")
    (set `self.TempX` (+ (`self.TempX`) _disttrace))
    (set `self.TempY` (+ (`self.TempY`) _disttrace))))

(fn `UserConstructionScript`
  (`BoxComponent.SetBoxExtent` (`self.Box`) (100.0 100.0 100.0) true))